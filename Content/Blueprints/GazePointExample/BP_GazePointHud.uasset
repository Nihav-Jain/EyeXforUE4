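; Example HUD that visualizes the eye tracker's gaze point as a colored square on screen.
; BeginPlay enables input so number keys switch the gaze point type between unfiltered and lightly filtered, and F10 toggles mouse emulation.
; DrawHUD prints a title with help text showing the active type, then draws the square centered on the gaze point whenever one is available.
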(event EventBeginPlay
  ;[1 1 1] Enable input for this blueprint
  (Input|EnableInput (Game|GetPlayerController 0)))

(event EventDrawHUD
  (params (SizeX :type Integer) (SizeY :type Integer))
  (bind _gazepointtype (Variables|Default|GetGazePointType))
  (bind _gazepointsize (Variables|Default|GetGazePointSize))
  (bind _returnvalue (/ _gazepointsize 2.0))
  (bind (_gazepoint _timestamp _bhasvalue) (Class|EyeXBlueprintLibrary|GetGazePoint _gazepointtype))
  (bind _returnvalue_2 (- _gazepoint _returnvalue))
  (bind (_x _y) (Math|Vector2D|BreakVector2D _returnvalue_2))
  ;[1 1 1] Print help message
  (bind (_screen_x _screen_y _outwidth _outheight) (Utilities|DrawCenteredTextonHUD (/ SizeX 2) (/ SizeY 3) "Eye-gaze point" "(R=1.000000,G=1.000000,B=1.000000,A=1.000000)" "/Game/Fonts/Calibri.Calibri" 1.0)
    (:%20%20
      (HUD|DrawText (Utilities|String|Append (Variables|Default|GetHelpText) (Utilities|String|EnumtoString (Variables|Default|GetGazePointType))) "(R=1.000000,G=1.000000,B=1.000000,A=1.000000)" _screen_x (+ _screen_y _outheight) "/Game/Fonts/Calibri_small.Calibri_small" 1.0 false)
      ;[1 1 1] Draw the gaze point on screen
      (if _bhasvalue
        (HUD|DrawRect "(R=0.985000,G=0.035203,B=0.814121,A=1.000000)" _x _y _gazepointsize _gazepointsize)))))

(event Input|KeyboardEvents|1
  ;[1 1 1] Set gaze point type on input
  (:Pressed
    (Variables|Default|SetGazePointType "Unfiltered")))

(event Input|KeyboardEvents|2
  ;[1 1 1] Set gaze point type on input
  (:Pressed
    (Variables|Default|SetGazePointType "LightlyFiltered")))

(event Input|KeyboardEvents|F10
  ;[1 1 1] Toggle mouse emulation
  (:Pressed
    (switch Utilities|FlowControl|Switch|SwitchonEEyeXEmulationMode (Class|EyeXBlueprintLibrary|GetEmulationMode)
      (:Disabled
        (Class|EyeXBlueprintLibrary|SetEmulationMode "Enabled"))
      (:Enabled
        (Class|EyeXBlueprintLibrary|SetEmulationMode "Disabled")))))

(fn ConstructionScript)