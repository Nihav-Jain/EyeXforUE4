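; Example actor that visualizes an eye tracker's 3D gaze point with a sphere component.
; Each tick it shows the sphere only while user presence is Present.
; When the user is present and a gaze point of the configured type is valid, it moves the sphere to that point, scaled by ten, in world space.
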(event EventTick
  (params (DeltaSeconds :type Float%20%28single-precision%29))
  (bind _userpresence (Class|EyeXBlueprintLibrary|GetUserPresence))
  (bind _gazepointtype (Variables|EyeX|GetGazePointType))
  (bind (_gazepoint _bhasvalue) (Class|EyeXBlueprintLibrary|Get3DGazePoint _gazepointtype))
  (bind _returnvalue (Utilities|Enum|Equal(Enum) _userpresence "Present"))
  ;[1 1 1] Move to the sphere to the position of the interpolated 3D gazepoint
  (Rendering|SetVisibility (Variables|Default|GetGazePointSPhere) _returnvalue false)
  (if (and _returnvalue _bhasvalue)
    (Transformation|SetWorldLocation (Variables|Default|GetGazePointSPhere) (* _gazepoint 1e+01) false)))

(fn ConstructionScript)